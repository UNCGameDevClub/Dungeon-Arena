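; First-person player character Blueprint that handles movement, mouse-look style camera control and gun use.
; On BeginPlay it adds a crosshair widget, spawns a BP_AutoRifle and snaps it to GunLocation as EquippedGun.
; Fire and reload inputs delegate to the gun, with shots aimed from the FPS camera along its forward vector to the gun's maximum bullet distance.
; Movement follows camera forward and right vectors, and vertical look input is inverted.
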(event EventBeginPlay
  ;[1 1 1] Spawn with gun
  (bind _returnvalue (UserInterface|CreateWidget "/Game/Widgets/Widget_Crosshair.Widget_Crosshair_C"))
  (UserInterface|Viewport|AddtoViewport _returnvalue 0)
  (bind _returnvalue_2 (Game|SpawnActorfromClass "/Game/Blueprints/GunBlueprints/BP_AutoRifle.BP_AutoRifle_C" (Variables|Default|GetNewVar_0) "Undefined" 0 0))
  (bind _output_get (Variables|Default|SetEquippedGun _returnvalue_2))
  (Transformation|AttachComponentToComponent _output_get (Variables|Default|GetGunLocation) "None" "SnapToTarget" "SnapToTarget" "KeepRelative" true))

(event Collision|EventActorBeginOverlap
  (params (OtherActor :type Actor%20Object%20Reference)))

(event EventTick
  (params (DeltaSeconds :type Float%20%28single-precision%29)))

(event Input|ActionEvents|InputActionReload
  (params (Key :type Key%20Structure))
  ;[1 1 1] Shooting
  (:Pressed
    (Default|Reload (Variables|Default|GetEquippedGun))))

(event Input|AxisEvents|InputAxisMove_Forward
  (params (AxisValue :type Float%20%28single-precision%29))
  ;[1 1 1] Character Movement
  (Pawn|Input|AddMovementInput (Math|Vector|GetForwardVector (Variables|Default|GetFPSCamera)) (* AxisValue (Variables|Default|GetMaxSpeed)) false))

(event Input|AxisEvents|InputAxisMove_Right
  (params (AxisValue :type Float%20%28single-precision%29))
  ;[1 1 1] Character Movement
  (Pawn|Input|AddMovementInput (Math|Vector|GetRightVector (Variables|Default|GetFPSCamera)) (* AxisValue (Variables|Default|GetMaxSpeed)) false))

(event Input|AxisEvents|InputAxisLookHorizontal
  (params (AxisValue :type Float%20%28single-precision%29))
  ;[1 1 1] Look Around
  (Pawn|Input|AddControllerYawInput AxisValue))

(event Input|AxisEvents|InputAxisLookVertical
  (params (AxisValue :type Float%20%28single-precision%29))
  ;[1 1 1] Look Around
  (Pawn|Input|AddControllerPitchInput (* AxisValue -1.0)))

(event Input|AxisEvents|InputAxisPrimary_Fire
  (params (AxisValue :type Float%20%28single-precision%29))
  (bind _fpscamera (Variables|Default|GetFPSCamera))
  (bind _equippedgun (Variables|Default|GetEquippedGun))
  (bind _returnvalue (Transformation|GetWorldLocation _fpscamera))
  ;[1 1 1] Shooting
  (if (== AxisValue 1.0)
    (Default|Shoot _equippedgun _returnvalue (+ _returnvalue (* (Math|Vector|GetForwardVector _fpscamera) (Variables|/Game/Blueprints/GunBlueprints/BP_BaseGun.BP_BaseGun_C|GetMaxBulletDistance (Variables|Default|GetEquippedGun)))))
    (else
      (Default|ReleaseTrigger _equippedgun))))

(fn ConstructionScript)