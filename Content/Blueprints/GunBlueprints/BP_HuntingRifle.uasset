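; BP_HuntingRifle is a single-shot hunting rifle weapon that overrides shooting from BP_SemiAutoRifle.
; Its construction script sets the magazine to one round and fills it.
; Shoot calls the parent shot, then waits for the reload speed delay and refills the magazine automatically.
; Reload passes straight to the parent implementation.
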(event EventBeginPlay
  (|CallParentFunction) ; This node is disabled and will not be called.\nDrag off pins to build functionality.
)

(event Collision|EventActorBeginOverlap
  (params (OtherActor :type Actor%20Object%20Reference))
  (|CallParentFunction OtherActor) ; This node is disabled and will not be called.\nDrag off pins to build functionality.
)

(event EventTick
  (params (DeltaSeconds :type Float%20%28single-precision%29))
  (|CallParentFunction DeltaSeconds) ; This node is disabled and will not be called.\nDrag off pins to build functionality.
)

(event EventShoot
  (params (StartPosition :type Vector :default "0, 0, 0") (EndPosition :type Vector :default "0, 0, 0"))
  ;[1 1 1] Override shooting from BP_SemiAutoRifle
  (|CallParentFunction StartPosition EndPosition)
  (Utilities|FlowControl|Delay (Variables|Default|GetReloadSpeed))
  (Variables|Default|SetCurrentMagazine (Variables|Default|GetMagazineSize)))

(event EventReload
  ;[1 1 1] Override shooting from BP_SemiAutoRifle
  (|CallParentFunction))

(fn ConstructionScript
  (|CallParentFunction)
  (Variables|Default|SetMagazineSize 1)
  (Variables|Default|SetCurrentMagazine (Variables|Default|GetMagazineSize)))