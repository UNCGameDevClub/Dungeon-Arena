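; BP_AutoRifle is a BP_BaseGun child that overrides Shoot to provide hitscan rifle fire.
; When CanShoot is set and the gun is automatic or the trigger was released, it line-traces on Visibility between the given points.
; A hit applies Damage, spawns a bullet decal, clears CanShoot and calls EventGunShot.
; A miss only clears IsReleased, so it skips both the CanShoot lock and the gunshot event.
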(event EventBeginPlay
  (|CallParentFunction) ; This node is disabled and will not be called.\nDrag off pins to build functionality.
)

(event Collision|EventActorBeginOverlap
  (params (OtherActor :type Actor%20Object%20Reference))
  (|CallParentFunction OtherActor) ; This node is disabled and will not be called.\nDrag off pins to build functionality.
)

(event EventTick
  (params (DeltaSeconds :type Float%20%28single-precision%29))
  (|CallParentFunction DeltaSeconds) ; This node is disabled and will not be called.\nDrag off pins to build functionality.
)

(event EventShoot
  (params (StartPosition :type Vector :default "0, 0, 0") (EndPosition :type Vector :default "0, 0, 0"))
  ;[1 1 1] Override Shoot function from BP_BaseGun
  (if (and (Variables|Default|GetCanShoot) (or (Variables|Default|GetIsAutomatic) (Variables|Default|GetisReleased)))
    (Variables|Default|SetisReleased false)
    (bind (_outhit _returnvalue) (Collision|LineTraceByChannel StartPosition EndPosition "TraceTypeQuery1" false 0 "None"))
    (if _returnvalue
      (Game|Damage|ApplyDamage (.HitActor (Collision|BreakHitResult _outhit)) (Variables|Default|GetDamage) 0 0)
      (bind _returnvalue_2 (Rendering|Decal|SpawnDecalatLocation "/Game/Materials/Material_BulletDecal.Material_BulletDecal" "2.000000,2.000000,2.000000" (.Location (Collision|BreakHitResult _outhit)) "-90.000000,0.000000,0.000000" 0.0))
      (Rendering|Components|Decal|SetFadeScreenSize _returnvalue_2 0.0)
      (Variables|Default|SetCanShoot false)
      (CallFunction|EventGunShot))))

(fn ConstructionScript
  (|CallParentFunction))