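; BP_BaseGun is a base gun Blueprint providing hitscan shooting with automatic or semi-automatic fire.
; Shoot line-traces between supplied points on the Visibility channel and, as placeholder debug behavior, spawns a bullet decal on hit.
; Only a hit starts the GunShot cooldown, which re-enables firing after the inverse of FireRate.
; ReleaseTrigger re-arms non-automatic guns for the next shot.
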(event Custom|Event%20GunShot
  (Utilities|FlowControl|Delay (/ 1.0 (Variables|Default|GetFireRate)))
  (Variables|Default|SetCanShoot true))

(event EventBeginPlay)

(event Collision|EventActorBeginOverlap
  (params (OtherActor :type Actor%20Object%20Reference)))

(event EventTick
  (params (DeltaSeconds :type Float%20%28single-precision%29)))

(fn ConstructionScript)

(fn Shoot
  (params (StartPosition :type Vector) (EndPosition :type Vector))
  (if (and (Variables|Default|GetCanShoot) (or (Variables|Default|GetIsAutomatic) (Variables|Default|GetisReleased)))
    (Variables|Default|SetisReleased false)
    ;[1 1 1] This block is debug code (it spawns a decal at hit location). Change it to fit specific implementation of gun
    (bind (_outhit _returnvalue) (Collision|LineTraceByChannel StartPosition EndPosition "TraceTypeQuery1" false 0 "None"))
    (if _returnvalue
      (bind _returnvalue_2 (Rendering|Decal|SpawnDecalatLocation "/Game/Blueprints/Material_BulletDecal.Material_BulletDecal" "2.000000,2.000000,2.000000" (.Location (Collision|BreakHitResult _outhit)) "-90.000000,0.000000,0.000000" 0.0))
      (Rendering|Components|Decal|SetFadeScreenSize _returnvalue_2 0.0)
      (Variables|Default|SetCanShoot false)
      (CallFunction|EventGunShot))))

(fn ReleaseTrigger
  (Variables|Default|SetisReleased true))